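; Breakable crystal actor that gets carved at a supplied location and falls apart into physics-simulated pieces, using Geometry Script.
; UpdateMesh forwards the location to a multicast event, which on first use swaps the static mesh for a dynamic mesh.
; Each cut boolean-subtracts a box from the tracked meshes, then splits them by connected components.
; One piece reuses the original component; others become new tracked components with generated collision.
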(event Custom|UpdateMesh_Multicast
  (params (NewParam :type Vector))
  (bind _dynamicmeshcomponent (Variables|Default|GetDynamicMeshComponent))
  (bind _dynamicmeshcomponent_2 (Variables|Default|GetDynamicMeshComponent))
  (if (Variables|Default|GetDynamicMeshEnabled)
    (for _array_element (Variables|Default|GetNewVar_0)
      (bind _returnvalue (DynamicMeshActor|AllocateComputeMesh))
      (bind _returnvalue_2 (Class|GeometryScriptLibraryMeshPrimitiveFunctions|AppendBox :TargetMesh _returnvalue :Origin "Center" :Debug 0))
      (bind _returnvalue_3 (DynamicMeshComponent|GetDynamicMesh _array_element))
      (bind _returnvalue_4 (GeometryScript|Booleans|ApplyMeshBoolean :TargetMesh _returnvalue_3 :TargetTransform (Transformation|GetActorTransform) :ToolMesh _returnvalue_2 :ToolTransform (Math|Transform|MakeTransform NewParam "0, 0, 0" "1.000000,1.000000,1.000000") :Operation "Subtract" :Debug 0))
      (bind _componentmeshes (Class|GeometryScriptLibraryMeshDecompositionFunctions|SplitMeshbyComponents _returnvalue_4 0 0))
      (Development|PrintString (Utilities|String|ToString(Integer) (Utilities|Array|Length _componentmeshes)))
      (for (_array_element_2 _array_index) _componentmeshes
        (if (== _array_index 1)
          (Class|DynamicMeshComponent|SetDynamicMesh _dynamicmeshcomponent_2 _array_element_2)
          (Physics|SetSimulatePhysics _dynamicmeshcomponent_2 true)
          (else
            (bind _returnvalue_5 (Game|AddComponentbyClass "/Script/GeometryFramework.DynamicMeshComponent" false))
            (Utilities|Array|Add (Variables|Default|GetNewVar_0) _returnvalue_5)
            (Collision|SetCollisionEnabled _returnvalue_5 "QueryAndPhysics")
            (Collision|SetCollisionResponsetoAllChannels (Variables|Default|GetDynamicMeshComponent) "ECR_Block")
            (Variables|/Script/GeometryFramework.DynamicMeshComponent|SetbEnableComplexCollision _returnvalue_5 true)
            (Class|DynamicMeshComponent|EnableComplexasSimpleCollision _returnvalue_5)
            (Class|DynamicMeshComponent|SetDynamicMesh _returnvalue_5 _array_element_2)
            (Class|GeometryScriptLibraryCollisionFunctions|SetDynamicMeshCollisionfromMesh _array_element_2 _returnvalue_5 (Utilities|Struct|MakeGeometryScriptCollisionfromMeshOptions true "MinVolumeShapes" true true true 1.0 true 25 0.1 "Z" true 100) 0)
            (Physics|SetSimulatePhysics _returnvalue_5 true)))))
    (else
      (bind _returnvalue_6 (DynamicMeshComponent|GetDynamicMesh _dynamicmeshcomponent))
      (bind _returnvalue_7 (DynamicMesh|Reset _returnvalue_6))
      (bind _returnvalue_8 (GeometryScript|StaticMesh|CopyMeshFromStaticMesh :FromStaticMeshAsset (Variables|/Script/Engine.StaticMeshComponent|GetStaticMesh (Variables|Character|GetMesh)) :ToDynamicMesh _returnvalue_7 :Debug 0)
        (:Success
          (Class|GeometryScriptLibraryCollisionFunctions|SetDynamicMeshCollisionfromMesh _returnvalue_8 (Variables|Default|GetDynamicMeshComponent) (Utilities|Struct|MakeGeometryScriptCollisionfromMeshOptions true "MinVolumeShapes") 0)
          (Class|DynamicMeshComponent|ConfigureMaterialSet _dynamicmeshcomponent (Rendering|Material|GetMaterials (Variables|Character|GetMesh)))
          (Variables|Default|SetDynamicMeshEnabled true)
          (Components|StaticMesh|SetStaticMesh (Variables|Character|GetMesh) 0)
          (bind _returnvalue_9 (DynamicMeshActor|AllocateComputeMesh))
          (bind _returnvalue_10 (Class|GeometryScriptLibraryMeshPrimitiveFunctions|AppendBox :TargetMesh _returnvalue_9 :Origin "Center" :Debug 0))
          (bind _returnvalue_11 (DynamicMeshComponent|GetDynamicMesh _array_element))
          (bind _returnvalue_12 (GeometryScript|Booleans|ApplyMeshBoolean :TargetMesh _returnvalue_11 :TargetTransform (Transformation|GetActorTransform) :ToolMesh _returnvalue_10 :ToolTransform (Math|Transform|MakeTransform NewParam "0, 0, 0" "1.000000,1.000000,1.000000") :Operation "Subtract" :Debug 0))
          (bind _componentmeshes_2 (Class|GeometryScriptLibraryMeshDecompositionFunctions|SplitMeshbyComponents _returnvalue_12 0 0))
          (Development|PrintString (Utilities|String|ToString(Integer) (Utilities|Array|Length _componentmeshes_2)))
          (for (_array_element_3 _array_index_2) _componentmeshes_2
            (if (== _array_index_2 1)
              (Class|DynamicMeshComponent|SetDynamicMesh _dynamicmeshcomponent_2 _array_element_3)
              (Physics|SetSimulatePhysics _dynamicmeshcomponent_2 true)
              (else
                (bind _returnvalue_13 (Game|AddComponentbyClass "/Script/GeometryFramework.DynamicMeshComponent" false))
                (Utilities|Array|Add (Variables|Default|GetNewVar_0) _returnvalue_13)
                (Collision|SetCollisionEnabled _returnvalue_13 "QueryAndPhysics")
                (Collision|SetCollisionResponsetoAllChannels (Variables|Default|GetDynamicMeshComponent) "ECR_Block")
                (Variables|/Script/GeometryFramework.DynamicMeshComponent|SetbEnableComplexCollision _returnvalue_13 true)
                (Class|DynamicMeshComponent|EnableComplexasSimpleCollision _returnvalue_13)
                (Class|DynamicMeshComponent|SetDynamicMesh _returnvalue_13 _array_element_3)
                (Class|GeometryScriptLibraryCollisionFunctions|SetDynamicMeshCollisionfromMesh _array_element_3 _returnvalue_13 (Utilities|Struct|MakeGeometryScriptCollisionfromMeshOptions true "MinVolumeShapes" true true true 1.0 true 25 0.1 "Z" true 100) 0)
                (Physics|SetSimulatePhysics _returnvalue_13 true)))))))))

(event EventBeginPlay
  (Utilities|Array|Add (Variables|Default|GetNewVar_0) (Variables|Default|GetDynamicMeshComponent)))

(event Collision|EventActorBeginOverlap
  (params (OtherActor :type Actor%20Object%20Reference)))

(event EventTick
  (params (DeltaSeconds :type Float%20%28single-precision%29)))

(event EventUpdateMesh
  (params (Location :type Vector :default "0, 0, 0") (Left :type Integer))
  (CallFunction|UpdateMeshMulticast Location))

(fn ConstructionScript)