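; BP_AppleTree is a growing resource tree that displays apples according to a remaining count.
; The construction script copies a static mesh into a dynamic mesh component, sets its material and collects four apple mesh slots into MeshArray.
; On BeginPlay, the authority starts a looping timer calling Grow, which is defined outside this file.
; UpdateMesh shows apples in slots below the Left count and clears the rest.
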(event Custom|GrowTimer
  (Development|PrintString "Hello")
  (Class|PlantResource|Grow))

(event EventBeginPlay
  (Networking|SwitchHasAuthority
    (:Authority
      (Utilities|Time|SetTimerbyFunctionName 0 "Grow" (Variables|Default|GetTimeToGrow) true))
    (:Remote
      (Development|PrintString "remote"))))

(event Collision|EventActorBeginOverlap
  (params (OtherActor :type Actor%20Object%20Reference)))

(event EventTick
  (params (DeltaSeconds :type Float%20%28single-precision%29)))

(event EventUpdateMesh
  (params (Location :type Vector :default "0, 0, 0") (Left :type Integer))
  (for (_array_element _array_index) (Variables|Default|GetMeshArray)
    (if (> Left _array_index)
      (Components|StaticMesh|SetStaticMesh _array_element "/Game/ResourcesAndTools/models/apple.apple")
      (else
        (Components|StaticMesh|SetStaticMesh _array_element 0)))))

(fn ConstructionScript
  (bind _returnvalue (DynamicMeshComponent|GetDynamicMesh (Variables|Default|GetDynamicMeshComponent)))
  (bind _returnvalue_2 (DynamicMesh|Reset _returnvalue))
  (GeometryScript|StaticMesh|CopyMeshFromStaticMesh :FromStaticMeshAsset (Variables|Default|GetStaticMesh) :ToDynamicMesh _returnvalue_2 :Debug 0
    (:Success
      (Class|DynamicMeshComponent|ConfigureMaterialSet (Variables|Default|GetDynamicMeshComponent) (Utilities|Array|MakeArray (Variables|Default|GetMaterial)))
      (Variables|Default|SetMeshArray (Utilities|Array|MakeArray (Variables|Default|GetStaticMesh1) (Variables|Default|GetStaticMesh2) (Variables|Default|GetStaticMesh3) (Variables|Default|GetStaticMesh4))))))