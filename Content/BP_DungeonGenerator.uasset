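; Dungeon generator Blueprint that supplies helpers for spawning resources on room surfaces, spawning characters and picking random numbers.
; SpawnResource traces along a random direction in the resource's cone and, on hitting the room, spawns the resource at the impact point.
; It orients the resource by summing mesh normals looked up from the hit face index.
; SpawnCharacter spawns a given race and returns its AICharacterController, printing an error if the cast fails.
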(event EventSpawnResource
  (params (ResourceInfo :type Resource%20Info%20Structure) (Center :type Vector :default "0, 0, 0") (Length :type Float%20%28single-precision%29) (Room :type Room%20Object%20Reference))
  (bind (_resourcetype _conedirection _coneangle) (Utilities|Struct|BreakResourceInfo ResourceInfo))
  (bind _outhit (Collision|LineTraceByChannel Center (+ Center (* (Math|Random|RandomUnitVectorinConeinDegrees _conedirection _coneangle) Length)) "TraceTypeQuery1" true 0 "None" false))
  (if (== (.HitActor (Collision|BreakHitResult _outhit)) Room)
    (bind (_vertices _triangles _normals _uvs _tangents) (Class|KismetProceduralMeshLibrary|GetSectionfromStaticMesh (Variables|/Script/Engine.StaticMeshComponent|GetStaticMesh (Variables|/Script/dungeon_wizard.Room|GetMesh Room))))
    (bind _returnvalue (Game|SpawnActorfromClass _resourcetype (Math|Transform|MakeTransform (.ImpactPoint (Collision|BreakHitResult _outhit)) (Math|Rotator|MakeRotfromZ (+ (Utilities|Array|Get(acopy) _normals (Utilities|Array|Get(acopy) _triangles (* (.FaceIndex (Collision|BreakHitResult _outhit)) 3))) (Utilities|Array|Get(acopy) _normals (+ (Utilities|Array|Get(acopy) _triangles (* (.FaceIndex (Collision|BreakHitResult _outhit)) 3)) 1)) (Utilities|Array|Get(acopy) _normals (+ (Utilities|Array|Get(acopy) _triangles (* (.FaceIndex (Collision|BreakHitResult _outhit)) 3)) 2)))) "1.000000,1.000000,1.000000") "AlwaysSpawn" 0 0))
    (Utilities|IsValid _returnvalue
      (:Is%20Not%20Valid
        (Development|PrintString "invalid")))))

(event EventTick
  (params (DeltaSeconds :type Float%20%28single-precision%29)))

(fn ConstructionScript
  (Transformation|SetActorRotation "0,10.000000, 0"))

(fn RandomFloat
  (params (Min :type Float%20%28single-precision%29) (Max :type Float%20%28single-precision%29))
  (return (Math|Random|RandomFloatinRange Min Max)))

(fn RandomInt
  (params (Min :type Integer) (Max :type Integer))
  (return (Math|Random|RandomIntegerinRange Min Max)))

(fn SpawnCharacter
  (params (Race :type Human%20Base%20Class%20Reference) (Location :type Vector :default "0, 0, 0"))
  (bind _returnvalue (Game|SpawnActorfromClass Race (Math|Transform|MakeTransform Location "0, 0, 0" "1.000000,1.000000,1.000000") "AdjustIfPossibleButAlwaysSpawn" 0 0))
  (bind _asaicharacter_controller (Utilities|Casting|CastToAICharacterController (AI|GetAIController _returnvalue))
    (:then
      (return _asaicharacter_controller))
    (:CastFailed
      (Development|PrintString "WRONG AICONTROLLER 
" true true "(R=1.000000,G=0.000000,B=0.040545,A=1.000000)" 1e+02))))