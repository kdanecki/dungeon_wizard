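; A test dynamic mesh actor that can be carved at runtime using Geometry Script booleans.
; The construction script resets the mesh to a large box and generates collision from it.
; Mine subtracts a pooled temporary sphere-box mesh at the passed location, rebuilds collision as convex hulls, then releases the compute meshes.
; Static mesh copy, solidify and simplify experiments remain disconnected.
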(event EventBeginPlay)

(event Collision|EventActorBeginOverlap
  (params (OtherActor :type Actor%20Object%20Reference)))

(event EventTick
  (params (DeltaSeconds :type Float%20%28single-precision%29)))

(fn ConstructionScript
  (bind _returnvalue (DynamicMeshComponent|GetDynamicMesh (Variables|DynamicMeshActor|GetDynamicMeshComponent)))
  (bind _returnvalue_2 (DynamicMesh|Reset _returnvalue))
  (bind _returnvalue_3 (Class|GeometryScriptLibraryMeshPrimitiveFunctions|AppendBox :TargetMesh _returnvalue_2 :DimensionX 5e+02 :DimensionY 5e+02 :DimensionZ 5e+02 :Debug 0))
  (Class|GeometryScriptLibraryCollisionFunctions|SetDynamicMeshCollisionfromMesh :FromDynamicMesh _returnvalue_3 :ToDynamicMeshComponent (Variables|DynamicMeshActor|GetDynamicMeshComponent) :Debug 0))

(fn Mine
  (params (NewParam :type Vector))
  (bind _returnvalue (DynamicMeshComponent|GetDynamicMesh (Variables|DynamicMeshActor|GetDynamicMeshComponent)))
  (bind _returnvalue_2 (DynamicMeshActor|AllocateComputeMesh))
  (bind _returnvalue_3 (Class|GeometryScriptLibraryMeshPrimitiveFunctions|AppendSphereBox :TargetMesh _returnvalue_2 :Transform (Math|Transform|MakeTransform NewParam "0, 0, 0" "1.000000,1.000000,1.000000") :Debug 0))
  (bind _returnvalue_4 (GeometryScript|Booleans|ApplyMeshBoolean :TargetMesh _returnvalue :ToolMesh _returnvalue_3 :Operation "Subtract" :Debug 0))
  (Class|GeometryScriptLibraryCollisionFunctions|SetDynamicMeshCollisionfromMesh _returnvalue_4 (Variables|DynamicMeshActor|GetDynamicMeshComponent) (Utilities|Struct|MakeGeometryScriptCollisionfromMeshOptions true "ConvexHulls" true true true 1.0 true 500 0.1 "Z" true 100) 0)
  (DynamicMeshActor|ReleaseAllComputeMeshes))