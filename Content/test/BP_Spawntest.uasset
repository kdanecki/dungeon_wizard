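; BP_Spawntest is a test actor that bulk-spawns BP_CrystalGreen actors, then removes them in timed batches.
; On BeginPlay it scatters about a thousand crystals in a spherical shell around itself, using random directions and distances, and stores them in an array.
; A looping five-second timer calls Spawn, which, despite its name, only destroys roughly 200 of the oldest entries, with no respawn or empty-array check.
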(event Custom|spawn
  (bind _newvar_0 (Variables|Default|GetNewVar_0))
  (for _index (range 0 200)
    (Actor|DestroyActor (Utilities|Array|Get(acopy) _newvar_0))
    (Utilities|Array|RemoveIndex _newvar_0)))

(event EventBeginPlay
  (for _index (range 0 1000)
    (bind _returnvalue (Game|SpawnActorfromClass "/Game/ResourcesAndTools/BP_CrystalGreen.BP_CrystalGreen_C" (Math|Transform|MakeTransform (+ (* (Math|Random|RandomUnitVector) (Math|Random|RandomFloatinRange 1e+03 1e+04)) (Transformation|GetActorLocation)) "0, 0, 0" "1.000000,1.000000,1.000000") "Undefined" 0 0))
    (Utilities|Array|Add (Variables|Default|GetNewVar_0) _returnvalue))
  (Utilities|Time|SetTimerbyEvent (delegate Custom|spawn) 5.0 true))

(event Collision|EventActorBeginOverlap
  (params (OtherActor :type Actor%20Object%20Reference)))

(event EventTick
  (params (DeltaSeconds :type Float%20%28single-precision%29)))

(fn ConstructionScript)