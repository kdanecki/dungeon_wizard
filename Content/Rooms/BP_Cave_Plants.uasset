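; Cave room actor that scatters apple trees and green crystals over its own mesh after a short delay on BeginPlay.
; SpawnThings fires random cone line traces, downward for trees and in any direction for crystals, and spawns only where they hit this actor.
; Each spawn is oriented by a vertex normal of the hit triangle, read from static mesh section data via the complex trace's face index.
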(event EventBeginPlay
  (|CallParentFunction)
  (Utilities|FlowControl|Delay 1e+01)
  (CallFunction|SpawnThings "/Game/ResourcesAndTools/BP_AppleTree.BP_AppleTree_C" 8e+01 20 "0, 0,-1.000000" "None")
  (CallFunction|SpawnThings "/Game/ResourcesAndTools/BP_CrystalGreen.BP_CrystalGreen_C" 1.8e+02 10 "0, 0,1.000000" "None"))

(event Collision|EventActorBeginOverlap
  (params (OtherActor :type Actor%20Object%20Reference))
  (|CallParentFunction OtherActor) ; This node is disabled and will not be called.\nDrag off pins to build functionality.
)

(event EventTick
  (params (DeltaSeconds :type Float%20%28single-precision%29))
  (|CallParentFunction DeltaSeconds) ; This node is disabled and will not be called.\nDrag off pins to build functionality.
)

(fn ConstructionScript
  (|CallParentFunction))

(fn SpawnThings
  (params (NewParam :type Actor%20Class%20Reference) (NewParam1 :type Float%20%28double-precision%29) (NewParam2 :type Integer) (NewParam3 :type Vector) (NewParam4 :type EDrawDebugTrace%20Enum :default "None"))
  (bind _returnvalue (Transformation|GetActorLocation))
  (for _index (range 0 (- NewParam2 1))
    (bind _outhit (Collision|LineTraceByChannel (+ _returnvalue "0,0,500.000000") (+ _returnvalue (* (Math|Random|RandomUnitVectorinConeinDegrees NewParam3 NewParam1) 3e+03)) "TraceTypeQuery1" true 0 NewParam4 false))
    (if (== (.HitActor (Collision|BreakHitResult _outhit)) self)
      (bind (_vertices _triangles _normals) (Class|KismetProceduralMeshLibrary|GetSectionfromStaticMesh (Variables|/Script/Engine.StaticMeshComponent|GetStaticMesh (Variables|Character|GetMesh))))
      (bind _returnvalue_2 (Game|SpawnActorfromClass NewParam (Math|Transform|MakeTransform (.ImpactPoint (Collision|BreakHitResult _outhit)) (Math|Rotator|MakeRotfromZ (Utilities|Array|Get(acopy) _normals (Utilities|Array|Get(acopy) _triangles (* (.FaceIndex (Collision|BreakHitResult _outhit)) 3)))) "1.000000,1.000000,1.000000") "AdjustIfPossibleButDontSpawnIfColliding" 0 0))
      (Utilities|IsValid _returnvalue_2
        (:Is%20Not%20Valid
          (Development|PrintString "invalid"))))))