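; BP_Cave3 is a cave room Blueprint that currently adds no active logic of its own.
; BeginPlay and the construction script only call the parent implementations, and the overlap event is disabled.
; Unconnected leftover nodes would add ItemSpawner components to ItemsToSpawn and spawn a BP_Goblin per entry, always at ItemSpawner8's location, but they never run.
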(event EventBeginPlay
  (|CallParentFunction))

(event Collision|EventActorBeginOverlap
  (params (OtherActor :type Actor%20Object%20Reference))
  (|CallParentFunction OtherActor) ; This node is disabled and will not be called.\nDrag off pins to build functionality.
)

(fn ConstructionScript
  (|CallParentFunction))