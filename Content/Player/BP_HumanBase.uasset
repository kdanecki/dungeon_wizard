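; Human base character for the player, handling inventory setup, hand items, combat, gathering and death.
; BeginPlay spawns a backpack into the inventory, Die drops both hand items, and CreateInventoryWidget opens the crafting UI.
; Tick line-traces from the camera along control rotation to store the looked-at actor and location.
; Attacks route through server and multicast montage events; attack and gather effects fire on montage notifies, and leftover debug chains remain unwired.
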(event Custom|Spawn
  (bind _returnvalue (Game|SpawnActorfromClass "/Game/ResourcesAndTools/BP_Backpack.BP_Backpack_C" (Transformation|GetActorTransform) "Undefined" 0 0))
  (Class|HumanBase|RightPickUp _returnvalue)
  (Class|HumanBase|ChangeItemContainer _returnvalue 3 0 1))

(event Custom|AttackAnimationMulticast
  (Animation|Montage|PlayMontage (Variables|Character|GetMesh) "/Game/Characters/AnimTest/AttackDown_Montage.AttackDown_Montage" 2.0))

(event Custom|AttackAnimationServer
  (params (Enemy :type Actor%20Object%20Reference) (Weapon :type Tool%20Object%20Reference))
  (CallFunction|AttackAnimationMulticast)
  (Animation|Montage|PlayMontage (Variables|Character|GetMesh) "/Game/Characters/AnimTest/AttackDown_Montage.AttackDown_Montage" 2.0
    (:OnNotifyBegin
      (Class|HumanBase|Attack Enemy Weapon))))

(event EventBeginPlay
  (|CallParentFunction)
  (CallFunction|Spawn))

(event EventAttackAnimation
  (params (Enemy :type Actor%20Object%20Reference) (Weapon :type Tool%20Object%20Reference))
  (Networking|SwitchHasAuthority
    (:Authority
      (CallFunction|AttackAnimationMulticast)
      (Animation|Montage|PlayMontage (Variables|Character|GetMesh) "/Game/Characters/AnimTest/AttackDown_Montage.AttackDown_Montage" 2.0
        (:OnNotifyBegin
          (Class|HumanBase|Attack Enemy Weapon))))
    (:Remote
      (CallFunction|AttackAnimationServer Enemy Weapon))))

(event EventTick
  (params (DeltaSeconds :type Float%20%28single-precision%29))
  (bind _camera (Variables|Default|GetCamera))
  (bind _outhit (Collision|LineTraceByChannel (Transformation|GetWorldLocation _camera) (+ (Transformation|GetWorldLocation _camera) (* (Math|Rotator|GetRotationXVector (Pawn|GetControlRotation :!class /Script/Engine.Pawn)) 1e+03)) "TraceTypeQuery2" true 0 "ForOneFrame"))
  (Variables|Default|SetLookingAt (.HitActor (Collision|BreakHitResult _outhit)))
  (Variables|Default|SetLookingAtLocation (.Location (Collision|BreakHitResult _outhit))))

(event EventCreateInventoryWidget
  (bind _returnvalue (Game|GetPlayerController 0))
  (bind _returnvalue_2 (Game|GetPlayerController 0))
  (Viewport|RemoveAllWidgets)
  (bind _returnvalue_3 (UserInterface|CreateWidget "/Game/Player/InventoryCraftingWidget.InventoryCraftingWidget_C" _returnvalue self))
  (Variables|/Game/Player/BP_PlayerController.BP_PlayerController_C|SetInventoryWidget (.AsBP%20Player%20Controller (Utilities|Casting|CastToBP_PlayerController _returnvalue)) _returnvalue_3)
  (UserInterface|Viewport|AddtoViewport _returnvalue_3 0)
  (Input|SetInputModeUIOnly _returnvalue_2 _returnvalue_3 "DoNotLock")
  (Variables|/Script/Engine.PlayerController|SetbShowMouseCursor _returnvalue_2 true))

(event EventGatherAnimation
  (params (Resource :type Natural%20Resource%20Object%20Reference) (Tool :type Tool%20Object%20Reference))
  (Animation|Montage|PlayMontage (Variables|Character|GetMesh) "/Game/Characters/AnimTest/AttackDown_Montage.AttackDown_Montage"
    (:OnNotifyBegin
      (Class|HumanBase|Gather Resource Tool))))

(event EventDie
  (if (not (Variables|Default|GetDead))
    (Variables|Default|SetDead true)
    (|CallParentFunction)
    (Collision|SetCollisionEnabled (Variables|Default|GetCapsuleComponent) "NoCollision")
    (Class|HumanBase|RightDrop)
    (Class|HumanBase|LeftDrop)))

(fn ConstructionScript)