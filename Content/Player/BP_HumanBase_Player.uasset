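; Player character Blueprint built on a parent class, handling the starting pickaxe and animated attacking and gathering.
; Spawn creates a pickaxe and picks it up in the right hand.
; Both actions share one montage: on its notify, attacks box-trace from the camera for BP_HumanBase actors or parents, while gathering requires still looking at the resource.
; Disconnected dynamic-mesh experiments (mining, booleans, simplification) never run.
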(event EventSpawn
  (bind _returnvalue (Game|SpawnActorfromClass "/Game/ResourcesAndTools/BP_Pickaxe.BP_Pickaxe_C" (Math|Transform|MakeTransform (+ (Transformation|GetActorLocation) "100.000000,0,100.000000") "0, 0, 0" "1.000000,1.000000,1.000000") "Undefined" 0 0))
  (Class|HumanBase|RightPickUp _returnvalue))

(event Collision|EventActorBeginOverlap
  (params (OtherActor :type Actor%20Object%20Reference)))

(event EventTick
  (params (DeltaSeconds :type Float%20%28single-precision%29))
  (|CallParentFunction DeltaSeconds))

(event EventAttackAnimation
  (params (Enemy :type Actor%20Object%20Reference) (Weapon :type Tool%20Object%20Reference))
  (bind _camera (Variables|Default|GetCamera))
  (bind _returnvalue (Transformation|GetWorldLocation _camera))
  (Animation|Montage|PlayMontage (Variables|Character|GetMesh) "/Game/Characters/AnimTest/AttackDown_Montage.AttackDown_Montage"
    (:OnNotifyBegin
      (bind _outhits (Class|KismetSystemLibrary|BoxTraceMulti _returnvalue (+ _returnvalue (* (Math|Rotator|GetRotationXVector (Pawn|GetControlRotation :!class /Script/Engine.Pawn)) 2e+03)) "50.000000,50.000000,50.000000" "0, 0, 0" "TraceTypeQuery3" true (Actor|GetAttachedActors true true) "None" true))
      (bind _array_element (Utilities|Array|ForEachLoopwithBreak _outhits :!label _label)
        (:LoopBody
          (bind _asbp_human_base (Utilities|Casting|CastToBP_HumanBase (.HitActor (Collision|BreakHitResult _array_element)))
            (:then
              (Class|HumanBase|Attack _asbp_human_base Weapon)
              (goto _label Break))
            (:CastFailed
              (bind _asbp_human_base_2 (Utilities|Casting|CastToBP_HumanBase (Actor|GetParentActor (.HitActor (Collision|BreakHitResult _array_element)))))
              (Class|HumanBase|Attack _asbp_human_base_2 Weapon))))))))

(event EventGatherAnimation
  (params (Resource :type Natural%20Resource%20Object%20Reference) (Tool :type Tool%20Object%20Reference))
  (Animation|Montage|PlayMontage (Variables|Character|GetMesh) "/Game/Characters/AnimTest/AttackDown_Montage.AttackDown_Montage"
    (:OnNotifyBegin
      (if (== Resource (Variables|Default|GetLookingAt))
        (Class|HumanBase|Gather Resource Tool)))))

(event EventDie
  (|CallParentFunction))

(fn ConstructionScript
  (|CallParentFunction))