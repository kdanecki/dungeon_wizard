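; Player controller that owns the on-screen game widget and keeps its display of Outcomes up to date.
; BeginPlay creates the widget and adds it to the viewport, and the OnRepOutcomes event tells it to refresh when valid.
; An unconnected leftover chain would rebuild the widget's outcomes box directly, adding a text entry with each item's resource type.
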(event Custom|AddWidget
  (bind _returnvalue (UserInterface|CreateWidget "/Game/Player/GameWidget.GameWidget_C" self))
  (Variables|Default|SetGameWidget _returnvalue)
  (UserInterface|Viewport|AddtoViewport _returnvalue 0))

(event EventBeginPlay
  (CallFunction|AddWidget))

(event EventOnRepOutcomes
  (bind _gamewidget (Variables|Default|GetGameWidget))
  (Utilities|IsValid _gamewidget
    (:Is%20Valid
      (Default|Refresh _gamewidget))))

(fn ConstructionScript)