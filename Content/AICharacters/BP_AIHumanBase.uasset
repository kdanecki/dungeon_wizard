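; BP_AIHumanBase is a base Blueprint for human AI characters that defines how their AI shuts down on death.
; Die stops the controller's brain logic, then, through AIC_CharacterBase, disables sight perception and removes that controller from its faction's member list.
; It then calls the parent Die; BeginPlay, Tick and overlap events are disabled stubs.
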(event EventBeginPlay
  (|CallParentFunction) ; This node is disabled and will not be called.\nDrag off pins to build functionality.
)

(event Collision|EventActorBeginOverlap
  (params (OtherActor :type Actor%20Object%20Reference)))

(event EventTick
  (params (DeltaSeconds :type Float%20%28single-precision%29))
  (|CallParentFunction DeltaSeconds) ; This node is disabled and will not be called.\nDrag off pins to build functionality.
)

(event EventDie
  (bind _self self)
  (bind _returnvalue (AI|GetAIController _self))
  (bind _asaic_character_base (Utilities|Casting|CastToAIC_CharacterBase _returnvalue))
  (AI|Logic|StopLogic (Variables|/Script/AIModule.AIController|GetBrainComponent _returnvalue) "")
  (Class|AIPerceptionComponent|SetSenseEnabled (Variables|/Game/AICharacters/AIC_CharacterBase.AIC_CharacterBase_C|GetAIPerception _asaic_character_base) "/Script/AIModule.AISense_Sight" false)
  (Utilities|Array|RemoveItem (Variables|/Script/dungeon_wizard.Faction|GetMembers (Variables|/Script/dungeon_wizard.AICharacterController|GetFaction _asaic_character_base)) _asaic_character_base)
  (|CallParentFunction))

(fn ConstructionScript
  (|CallParentFunction))